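; Scatter-shot weapon for Bird of Prey that fans its projectiles evenly across a horizontal arc centred on the weapon's facing.
; It overrides only the projectile spawn transform, placing every shot at the actor's location and keeping its roll and pitch.
; Yaw steps from one arc edge to the other using ArcAngle, NumShots and a 1-based ShotNumber, with no guard against a single-shot divide by zero.
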(event EventBeginPlay)

(event Collision|EventActorBeginOverlap
  (params (OtherActor :type Actor%20Object%20Reference)))

(event EventTick
  (params (DeltaSeconds :type Float%20%28single-precision%29)))

(fn ConstructionScript
  (|CallParentFunction))

(fn GetProjectileSpawnTransform
  (params (Shot%20Number :type Integer))
  (bind _returnvalue (Transformation|GetActorRotation))
  (bind (_roll _pitch _yaw) (Math|Rotator|BreakRotator _returnvalue))
  (return (Math|Transform|MakeTransform (Transformation|GetActorLocation) (Math|Rotator|MakeRotator _roll _pitch (+ (- _yaw (/ (Variables|Default|GetArcAngle) 2.0)) (* (- Shot%20Number 1) (/ (Variables|Default|GetArcAngle) (Math|Conversions|ToFloat(Integer) (- (Variables|Default|GetNumShots) 1)))))) "1,1,1")))