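; BasePowerUp is the base pickup actor for player ship power-ups in BirdOfPrey.
; When a PlayerShip overlaps it, it calls Apply, an empty hook here, plays a fixed pickup sound and destroys itself.
; A Reset event also destroys the actor.
; PlayEffects spawns a configurable particle and sound at its location, but nothing in this Blueprint calls it.
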(event Collision|EventActorBeginOverlap
  (params (OtherActor :type Actor%20Object%20Reference))
  ;[1 1 1] Pick up on overlap
  (bind _asplayer_ship (Utilities|Casting|CastToPlayerShip OtherActor))
  (CallFunction|Apply _asplayer_ship)
  (Audio|PlaySoundatLocation "/Game/BirdOfPrey/UI/PickupItem_Cue.PickupItem_Cue" (Transformation|GetActorLocation))
  (Actor|DestroyActor))

(event EventReset
  ;[1 1 1] Handle Reset
  (Actor|DestroyActor))

(fn ConstructionScript)

(fn Apply
  (params (PlayerShip :type Player%20Ship%20Object%20Reference)))

(fn PlayEffects
  (Effects|SpawnEmitteratLocation (Variables|Effects|GetPickUpParticleSystem) (Transformation|GetActorLocation))
  (Audio|PlaySoundatLocation (Variables|Effects|GetPickUpSoundCue) (Transformation|GetActorLocation)))