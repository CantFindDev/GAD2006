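; BaseWeapon is the parent weapon actor for BirdOfPrey, defining a common firing interface with placeholder defaults for child Blueprints to override.
; StartFire and StopFire are empty, IsFiring returns false and HasFinishedFiring returns true.
; PlayFireEffects, the shared helper, spawns the fire particle attached to the root at GetFireEffectSpawnTransform, which defaults to the actor's location and rotation, and plays the fire sound.
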(event EventBeginPlay)

(event Collision|EventActorBeginOverlap
  (params (OtherActor :type Actor%20Object%20Reference)))

(event EventTick
  (params (DeltaSeconds :type Float%20%28single-precision%29)))

(fn ConstructionScript)

(fn StartFire)

(fn StopFire)

(fn PlayFireEffects
  (bind _returnvalue (CallFunction|GetFireEffectSpawnTransform))
  (bind (_location _rotation) (Math|Transform|BreakTransform _returnvalue))
  (Effects|SpawnEmitterAttached (Variables|Effects|GetFireParticleEffect) (Variables|Default|GetDefaultSceneRoot) "None" _location _rotation "1.000000,1.000000,1.000000" "KeepWorldPosition")
  (Audio|PlaySoundatLocation (Variables|Effects|GetFireSoundCue) (Transformation|GetActorLocation)))

(fn GetFireEffectSpawnTransform
  (return (Math|Transform|MakeTransform (Transformation|GetActorLocation) (Transformation|GetActorRotation) "1,1,1")))

(fn HasFinishedFiring
  (return true))

(fn IsFiring
  (return false))